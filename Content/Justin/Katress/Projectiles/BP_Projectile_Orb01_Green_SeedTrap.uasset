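; Green seed trap orb projectile for Katress, with an Explode event that handles its impact effect and shutdown.
; Explode applies the colored hit VFX, deactivates the projectile and spawns an emitter by SeedTrapState, five times larger when Landed than when Launched or Dispersed.
; It then disables sphere collision, leaves the actor unhidden and sets a short lifespan for delayed destruction.
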(event EventBeginPlay
  (|CallParentFunction))

(event Collision|EventActorBeginOverlap
  (params (OtherActor :type Actor%20Object%20Reference))
  (|CallParentFunction OtherActor))

(event EventTick
  (params (DeltaSeconds :type Float%20%28single-precision%29))
  (|CallParentFunction DeltaSeconds))

(event EventExplode
  (bind _returnvalue (Transformation|GetActorTransform))
  (bind _returnvalue_2 (Transformation|GetActorTransform))
  (Effects|Components|ParticleSystem|SetTemplate (Variables|Default|GetHit) (Variables|Default|GetVFXHit/Impact))
  (Effects|Components|ParticleSystem|SetColorParameter (Variables|Default|GetHit) "Color" (Variables|Default|GetColor))
  (Transformation|SetWorldLocation (Variables|Default|GetHit) (Transformation|GetActorLocation) false false)
  (Components|Activation|Deactivate (Variables|Default|GetProjectile))
  (switch Utilities|FlowControl|Switch|SwitchonESeedTrapState (Variables|Default|GetSeedTrapState)
    (:LAUNCHED
      (Effects|SpawnEmitteratLocation (Variables|/Script/Engine.ParticleSystemComponent|GetTemplate (Variables|Default|GetHit)) (.location _returnvalue) (.rotation _returnvalue) (.scale _returnvalue) :!label _label))
    (:DISPERSE
      (goto _label))
    (:LANDED
      (Effects|SpawnEmitteratLocation (Variables|/Script/Engine.ParticleSystemComponent|GetTemplate (Variables|Default|GetHit)) (.location _returnvalue_2) (.rotation _returnvalue_2) (* (.scale _returnvalue_2) 5.0))))
  (Collision|SetCollisionEnabled (Variables|Default|GetSphereComp) "NoCollision")
  (Rendering|SetActorHiddenInGame false)
  (Actor|SetLifeSpan 5.0))

(fn ConstructionScript
  (|CallParentFunction))