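; Ignis Blast projectile actor with configurable particle effects for muzzle, flight and hit, whose speed, spin, color and scale are applied in the construction script.
; BeginPlay shows the muzzle and, given a warm-up time, hides and halts the projectile before relaunching it.
; On overlap it calls the parent handler, plays impact sound and effects, then destroys itself immediately.
; The looping respawn and delayed-destroy chains are disconnected.
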(event Custom|SpawnMuzzle
  (bind _muzzle (Variables|Default|GetMuzzle))
  ;[1 0 0] Move these to c++
  (Effects|Components|ParticleSystem|SetTemplate _muzzle (Variables|Default|GetVFXMuzzle))
  (Transformation|SetWorldLocation _muzzle (+ (Transformation|GetActorLocation) (Variables|Default|GetMuzzleOffset)) false false))

(event Custom|SpawnProjectile
  ;[1 0 0] Move these to c++
  (Effects|Components|ParticleSystem|SetTemplate (Variables|Default|GetProjectile) (Variables|Default|GetVFXProjectile))
  (Game|Components|ProjectileMovement|SetVelocityinLocalSpace (Variables|Default|GetProjectileMovement) (Variables|Default|GetoriginalVelocity)))

(event Custom|StopProjectile
  ;[1 0 0] Move these to c++
  (Components|Activation|Deactivate (Variables|Default|GetProjectile))
  (Components|Movement|StopMovementImmediately (Variables|Default|GetProjectileMovement)))

(event Custom|SetProjectileTemplateToEmpty
  ;[1 0 0] Move these to c++
  (Effects|Components|ParticleSystem|SetTemplate (Variables|Default|GetProjectile) 0)
  (Components|Movement|StopMovementImmediately (Variables|Default|GetProjectileMovement)))

(event EventBeginPlay
  (bind _warmuptime (Variables|Default|GetWarmUpTime))
  ;[1 0 0] Move these to c++
  (Variables|Default|SetoriginalVelocity (Variables|/Script/Engine.MovementComponent|GetVelocity (Variables|Default|GetProjectileMovement)))
  (Variables|Default|SetoriginalLocation (Transformation|GetWorldLocation (Variables|Default|GetSphereComp)))
  (CallFunction|SpawnMuzzle)
  (if (> _warmuptime 0.0)
    (CallFunction|SetProjectileTemplatetoEmpty)
    (Utilities|FlowControl|Delay _warmuptime)
    (CallFunction|SpawnProjectile)))

(event EventOnOverlapBegin
  (params (OverlappedComponent :type Primitive%20Component%20Object%20Reference) (OtherActor :type Actor%20Object%20Reference) (OtherComp :type Primitive%20Component%20Object%20Reference) (OtherBodyIndex :type Integer) (bFromSweep :type Boolean) (SweepResult :type Hit%20Result%20Structure%20%28by%20ref%29))
  (bind _returnvalue (Transformation|GetActorTransform))
  (bind _hit (Variables|Default|GetHit))
  ;[1 0 0] Move these to c++
  (|CallParentFunction OverlappedComponent OtherActor OtherComp OtherBodyIndex bFromSweep SweepResult)
  (Audio|PlaySoundatLocation "/Game/Assets/Sounds/IgnisBlast/IgnisBlast_Impact01_Cue.IgnisBlast_Impact01_Cue" (Transformation|GetActorLocation OtherActor) "0, 0, 0" 1.0 1.0 0.0 0 0 0 0)
  (Effects|Components|ParticleSystem|SetTemplate _hit (Variables|Default|GetVFXHit/Impact))
  (Transformation|SetWorldLocation _hit (+ (Math|Transform|TransformLocation (Transformation|GetActorTransform) "0, 0, 0") (Variables|Default|GetHit/ImpactOffset)) false false)
  (CallFunction|StopProjectile)
  (Effects|SpawnEmitteratLocation (Variables|/Script/Engine.ParticleSystemComponent|GetTemplate (Variables|Default|GetHit)) (.location _returnvalue) (.rotation _returnvalue) (* (.scale _returnvalue) 1.5))
  (Actor|DestroyActor))

(event EventTick
  (params (DeltaSeconds :type Float%20%28single-precision%29)))

(fn ConstructionScript
  (bind _scale (Variables|Default|GetScale))
  (bind _scale_2 (Variables|Default|GetScale))
  (bind _projectile (Variables|Default|GetProjectile))
  (bind _scale_3 (Variables|Default|GetScale))
  (bind _hit (Variables|Default|GetHit))
  (bind _muzzle (Variables|Default|GetMuzzle))
  (bind _color (Variables|Default|GetColor))
  (Variables|/Script/Engine.ProjectileMovementComponent|SetInitialSpeed (Variables|Default|GetProjectileMovement) (Variables|Default|GetProjectileSpeed))
  (Effects|Components|ParticleSystem|SetTemplate (Variables|Default|GetProjectile) (Variables|Default|GetVFXProjectile))
  (Variables|/Script/Engine.RotatingMovementComponent|SetRotationRate (Variables|Default|GetRotatingMovement) (Variables|Default|GetRotationRate))
  (if (Variables|Default|GetChangeColor%20?)
    (Effects|Components|ParticleSystem|SetColorParameter (Variables|Default|GetProjectile) "Color" _color)
    (Effects|Components|ParticleSystem|SetColorParameter (Variables|Default|GetHit) "Color" _color)
    (Effects|Components|ParticleSystem|SetColorParameter (Variables|Default|GetMuzzle) "Color" _color))
  (Effects|Components|ParticleSystem|SetVectorParameter _projectile "Scale" _scale_2)
  (Effects|Components|ParticleSystem|SetFloatParameter _projectile "Scale" (.X (Math|Vector|BreakVector _scale_2)))
  (Effects|Components|ParticleSystem|SetVectorParameter _hit "Scale" _scale_3)
  (Effects|Components|ParticleSystem|SetFloatParameter _hit "Scale" (.X (Math|Vector|BreakVector _scale_3)))
  (Effects|Components|ParticleSystem|SetVectorParameter _muzzle "Scale" _scale)
  (Effects|Components|ParticleSystem|SetFloatParameter _muzzle "Scale" (.X (Math|Vector|BreakVector _scale))))