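; BP_Bolt2 is a short-lived homing bolt skill projectile that damages what it hits.
; On BeginPlay it homes on the root component of the Target held by its owner's GrizzBoltActorComponent, then destroys itself after a brief delay.
; A mesh overlap with any actor other than the owner applies random damage in a fixed range through ApplyDamage and destroys the bolt.
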(event OnComponentBeginOverlap(MeshComp)
  (params (OverlappedComponent :type Primitive%20Component%20Object%20Reference) (OtherActor :type Actor%20Object%20Reference) (OtherComp :type Primitive%20Component%20Object%20Reference) (OtherBodyIndex :type Integer) (bFromSweep :type Boolean) (SweepResult :type Hit%20Result%20Structure%20%28by%20ref%29))
  (bind _returnvalue (Components|GetOwner))
  (if (!= OtherActor _returnvalue)
    (Class|PStatusLibrary|ApplyDamage _returnvalue OtherActor (Math|Random|RandomFloatinRange 5e+01 1e+02))
    (Actor|DestroyActor)))

(event EventBeginPlay
  (Variables|/Script/Engine.ProjectileMovementComponent|SetHomingTargetComponent (Variables|Default|GetProjectileMovementComponent) (Variables|/Script/Engine.Actor|GetRootComponent (Variables|/Script/Pal_World.GrizzBoltActorComponent|GetTarget (Actor|GetComponentbyClass (Components|GetOwner) "/Script/Pal_World.GrizzBoltActorComponent"))))
  (Utilities|FlowControl|Delay 1.2)
  (Actor|DestroyActor))

(event Collision|EventActorBeginOverlap
  (params (OtherActor :type Actor%20Object%20Reference)))

(event EventTick
  (params (DeltaSeconds :type Float%20%28single-precision%29)))

(fn ConstructionScript)