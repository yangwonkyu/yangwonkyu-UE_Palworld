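; Blueprint that attaches a Niagara trail effect to a character's skeletal mesh when Call_Trail_8 runs.
; It spawns the P_Trail_7 system, despite the Trail_8 name, and binds the mesh to its Skeletal Mesh user parameter.
; A looping timer then feeds the system the character's movement speed and a scaled, backward-facing direction from the capsule.
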(event Custom|Call_Trail_8
  (bind _character (Variables|Default|GetCharacter))
  (bind _mesh (Variables|/Script/Engine.Character|GetMesh _character))
  ;[0 0.1821 1] Apply the effect to the get skeletal mesh
  (bind _returnvalue (Niagara|SpawnSystemAttached "/Game/NiagaraCharacterTrail/Niagara/P_Trail_7.P_Trail_7" _mesh "None" "0, 0, 0" "0, 0, 0" "KeepRelativeOffset" false))
  (Class|NiagaraFunctionLibrary|OverrideSystemUserVariableSkeletalMeshComponent _returnvalue "Skeletal Mesh" _mesh)
  (Utilities|Time|SetTimerbyEvent (delegate Custom|Tick) 0.1 true))

(event Custom|Tick
  (bind _character (Variables|Default|GetCharacter))
  ;[0 0.1821 1] Apply the effect to the get skeletal mesh
  (Niagara|SetNiagaraVariable(Float) (stale Custom|Call_Trail_8 _returnvalue) "V" (Math|Vector|VectorLength (Variables|/Script/Engine.MovementComponent|GetVelocity (Variables|/Script/Engine.Character|GetCharacterMovement _character))))
  (Niagara|SetNiagaraVariable(Vector3) (stale Custom|Call_Trail_8 _returnvalue) "Direction" (* (Math|Vector|GetForwardVector (Variables|/Script/Engine.Character|GetCapsuleComponent _character)) -5e+01)))